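; Pattern manager that periodically triggers randomly chosen sets of BP_DisappearPlatform platforms with escalating difficulty.
; A looping timer picks one of fifteen predefined pattern arrays and calls each element's event with the current DT_Difficulty row.
; Difficulty rises after each launch, clamped to four levels.
; When GM_Character flags GameFinished, that tick resets difficulty and clears the flag instead of launching a pattern.
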(event `self.ReceiveBeginPlay`
  ;[0.04154 0.01876 0.4167] PatternSystem
  (bind _outactors (`GameplayStatics.GetAllActorsOfClass` "/Game/Thomas/BPs/DIsappearPlatform/BP_DisappearPlatform.BP_DisappearPlatform_C"))
  (set `self.Platforms` _outactors)
  (`KismetSystemLibrary.K2_SetTimerDelegate` (delegate `SystemPattern`) (`self.Changement`) true))

(event `SystemPattern`
  ;[0.04154 0.01876 0.4167] PatternSystem
  (bind _asgm_character (cast `/Game/Thomas/BPs/GM_Character` (`GameplayStatics.GetGameMode`)))
  (if (`/Game/Thomas/BPs/GM_Character.GameFinished` _asgm_character)
    (set `self.Difficulty` 1)
    (set `/Game/Thomas/BPs/GM_Character.GameFinished` false _asgm_character)
    (else
      (`self.EventLaunchPattern` (select `int` (`KismetMathLibrary.RandomIntegerInRange` 0 14) :`0` (`self.Pattern001`) :`1` (`self.Pattern002`) :`2` (`self.Pattern003`) :`3` (`self.Pattern004`) :`4` (`self.Pattern005`) :`5` (`self.Pattern006`) :`6` (`self.Pattern007`) :`7` (`self.Pattern008`) :`8` (`self.Pattern009`) :`9` (`self.Pattern010`) :`10` (`self.Pattern011`) :`11` (`self.Pattern012`) :`12` (`self.Pattern013`) :`13` (`self.Pattern014`) :`14` (`self.Pattern015`)))
      (set `self.Difficulty` (`KismetMathLibrary.Clamp` (+ (`self.Difficulty`) 1) 1 4)))))

(event `EventLaunchPattern`
  (params (Array :type "Array of /Game/Thomas/BPs/DIsappearPlatform/BP_DisappearPlatform Object Reference (by ref)"))
  ;[0 0.2969 0.05615] PatternList
  (bind _returnvalue (`|GetDataTableRow` "/Game/DT_Difficulty.DT_Difficulty" (`KismetStringLibrary.Conv_StringToName` (`KismetStringLibrary.Concat_StrStr` "difficulty" (`KismetStringLibrary.Conv_IntToString` (`self.Difficulty`)))))
    (:`then`
      (set `self.ActualDifficultyValues` _returnvalue)
      (for _array_element Array
        (`/Game/Thomas/BPs/DIsappearPlatform/BP_DisappearPlatform.Event` _array_element (`self.ActualDifficultyValues`))))))

(fn `UserConstructionScript`)