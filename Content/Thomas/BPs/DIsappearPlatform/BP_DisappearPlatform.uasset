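; Disappearing platform that, when its event is called, shakes, drops away, then rises back as solid ground.
; A timeline jitters the cube orange, alternating random offsets with resets to its starting position via FlipFlop.
; A second timeline lowers it red without collision, waits, then reverses, restoring collision and turning it green.
; The event's parameter sets both timelines' durations and the delay; an older material-flicker version remains unwired.
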(event `Event`
  (params (NewParam :type "/Game/STileInfos Structure"))
  (bind _minoffset (`self.MinOffset`))
  (bind _maxoffset (`self.MaxOffset`))
  (`MeshComponent.SetVectorParameterValueOnMaterials` (`self.Cube`) "Color" (`KismetMathLibrary.Conv_LinearColorToVector` (struct :`R` 1.0 :`G` 0.633787 :`A` 1.0)))
  (`TimelineComponent.SetPlayRate` (`self.PlatformShaking`) (/ 1.0 NewParam_TimeShaking_2_D31ADFE046644262D2315DB0781C3A8C))
  (bind (_direction _shakingvalue) (`Timeline|PlatformShaking` :!via `PlayFromStart`)
    (:`Update`
      (`/Engine/EditorBlueprintResources/StandardMacros.FlipFlop`
        (:`A`
          (`SceneComponent.K2_AddLocalOffset` (`self.Cube`) (`KismetMathLibrary.MakeVector` (* _shakingvalue (`KismetMathLibrary.RandomFloatInRange` _minoffset _maxoffset)) (* _shakingvalue (`KismetMathLibrary.RandomFloatInRange` _minoffset _maxoffset))) false false))
        (:`B`
          (`SceneComponent.K2_SetRelativeLocation` (`self.Cube`) (`self.InitialRelativeLocation`) false false))))
    (:`Finished`
      (`SceneComponent.K2_SetRelativeLocation` (`self.Cube`) (`self.InitialRelativeLocation`) false false)
      (`MeshComponent.SetVectorParameterValueOnMaterials` (`self.Cube`) "Color" (`KismetMathLibrary.Conv_LinearColorToVector` (struct :`R` 1.0 :`B` 0.101925 :`A` 1.0)))
      (`PrimitiveComponent.SetCollisionEnabled` (`self.Cube`) "NoCollision")
      (`TimelineComponent.SetPlayRate` (`self.Falling`) (/ 1.0 NewParam_TimeFalling_4_218A1848495FE4F18B15388EFF8D26DB))
      (bind (_direction_2 _newtrack_0) (`Timeline|Falling` :!via `PlayFromStart` :!label _label)
        (:`Update`
          (`SceneComponent.K2_SetRelativeLocation` (`self.Cube`) (`KismetMathLibrary.MakeVector` 0.0 0.0 (`KismetMathLibrary.Lerp` -117.0 -500.0 _newtrack_0)) false false))
        (:`Finished`
          (switch `ETimelineDirection` _direction_2
            (:`Forward`
              (`KismetSystemLibrary.Delay` NewParam_DelayUp_7_E8F688A94E97D145446773AD1CBABA8E)
              (goto _label :!via `Reverse`))
            (:`Backward`
              (`MeshComponent.SetVectorParameterValueOnMaterials` (`self.Cube`) "Color" (`KismetMathLibrary.Conv_LinearColorToVector` (struct :`R` 0.035294 :`G` 0.701961 :`A` 1.0)))
              (`PrimitiveComponent.SetCollisionEnabled` (`self.Cube`) "QueryAndPhysics"))))))))

(event `self.ReceiveBeginPlay`
  (set `self.InitialRelativeLocation` (`SceneComponent.RelativeLocation` (`self.Cube`))))

(fn `UserConstructionScript`)