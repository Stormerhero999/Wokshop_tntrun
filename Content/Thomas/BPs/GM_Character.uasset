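; Game mode for a local multiplayer last-player-standing game, with rounds hard-coded for four players.
; BeginPlay creates local players, possesses characters spawned at tagged PlayerStarts, sets player 0's view to BP_Cam, and loops timers spawning random bonuses and jack-in-the-boxes on disappearing platforms.
; Tick polls the death count to score a lone survivor or handle a draw.
; FInishedGame then shows the win screen at three points or teleports characters back after a delay.
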(event `FInishedGame`
  (bind _outactors (`GameplayStatics.GetAllActorsOfClass` "/Game/Thomas/BPs/BP_Character.BP_Character_C"))
  (for _array_element _outactors
    (if (== (`/Game/Thomas/BPs/BP_Character.Score` _array_element) 3)
      (bind _returnvalue (`|CreateWidget` "/Game/Thomas/BPs/WIn.WIn_C"))
      (`UserWidget.AddToViewport` _returnvalue 0)
      (set `self.GameFinished` true)
      (set `PlayerController.bShowMouseCursor` true (`GameplayStatics.GetPlayerController` 0))
      (`GameplayStatics.SetGamePaused` true)
      (else
        (set `self.GameFinished` true)
        (`KismetSystemLibrary.Delay` 4.0)
        (bind _outactors_2 (`GameplayStatics.GetAllActorsOfClass` "/Game/Thomas/BPs/BP_Character.BP_Character_C"))
        (for (_array_element_2 _array_index) _outactors_2
          (`self.K2_TeleportTo` :`self` _array_element_2 :`DestLocation` (`self.K2_GetActorLocation` (`|GetArrayItem` (`self.PlayerStart`) _array_index)))
          (set `self.nbpersondead` 0))))))

(event `self.ReceiveTick`
  (params (DeltaSeconds :type "Float (single-precision)"))
  (if (== (`self.nbpersondead`) 3)
    (`/Engine/EditorBlueprintResources/StandardMacros.DoOnce` false :!label _label
      (:`Completed`
        (bind _outactors (`GameplayStatics.GetAllActorsOfClass` "/Game/Thomas/BPs/BP_Character.BP_Character_C"))
        (for _array_element _outactors
          (if (not (`/Game/Thomas/BPs/BP_Character.PlayerDead` _array_element))
            (`/Engine/EditorBlueprintResources/StandardMacros.IncrementInt` (`/Game/Thomas/BPs/BP_Character.Score` _array_element)
              (:`  `
                (bind _returnvalue (`|CreateWidget` "/Game/Thomas/BPs/WBP_UserInteface.WBP_UserInteface_C"))
                (`UserWidget.AddToViewport` _returnvalue 0)
                (set `self.nbpersondead` 0)
                (`self.FInishedGame`)
                (goto _label :!via `Reset`)))))))
    (elif (== (`self.nbpersondead`) 4)
      (`/Engine/EditorBlueprintResources/StandardMacros.DoOnce` false :!label _label_2
        (:`Completed`
          (bind _returnvalue_2 (`|CreateWidget` "/Game/Thomas/BPs/WBP_UserInteface.WBP_UserInteface_C"))
          (`UserWidget.AddToViewport` _returnvalue_2 0)
          (set `self.nbpersondead` 0)
          (`self.FInishedGame`)
          (goto _label_2 :!via `Reset`))))))

(event `self.ReceiveBeginPlay`
  (bind _outactors (`GameplayStatics.GetAllActorsOfClass` "/Script/Engine.PlayerStart"))
  (set `self.PlayerStart` _outactors)
  (bind _returnvalue (`|SpawnActorFromClass` "/Game/Thomas/BPs/BP_Character.BP_Character_C" (`self.GetTransform` (`self.FindPlayerStartByTag` 1)) "Undefined" "OverrideRootScale" null 0 null))
  (`Controller.Possess` (`GameplayStatics.GetPlayerController` 0) _returnvalue)
  ;[1 0.4927 0.02567] MultiplayerSystem
  (`|ExecutionSequence`
    (:`then_0`
      (for _index (range 1 (`self.NbPlayerToSpawn`))
        (bind _returnvalue_2 (`GameplayStatics.GetPlayerControllerFromID` _index))
        (`/Engine/EditorBlueprintResources/StandardMacros.IsValid` _returnvalue_2
          (:`Is Valid`
            _)
          (:`Is Not Valid`
            (`GameplayStatics.CreatePlayer` _index)))
        (bind _returnvalue_3 (`|SpawnActorFromClass` "/Game/Thomas/BPs/BP_Character.BP_Character_C" (`self.GetTransform` (`self.FindPlayerStartByTag` (+ _index 1))) "Undefined" "OverrideRootScale" null _index null))
        (`Controller.Possess` _returnvalue_2 _returnvalue_3))
      (bind _returnvalue_4 (`GameplayStatics.GetActorOfClass` "/Game/Thomas/BPs/BP_Cam.BP_Cam_C"))
      (`PlayerController.SetViewTargetWithBlend` (`GameplayStatics.GetPlayerController` 0) _returnvalue_4 0.0 "VTBlend_Linear" 0.0 false))
    (:`then_1`
      ;[0.9795 0 1] SpawnBonusSystem
      (`KismetSystemLibrary.K2_SetTimerDelegate` (delegate `SpawnBonus`) 10.0 true))
    (:`then_2`
      ;[0.376 0 0.03951] JACK EVENT
      (`KismetSystemLibrary.K2_SetTimerDelegate` (delegate `SpawnJACK`) 10.0 true))))

(event `SpawnBonus`
  ;[0.9795 0 1] SpawnBonusSystem
  (bind _outactors (`GameplayStatics.GetAllActorsOfClass` "/Game/Thomas/BPs/DIsappearPlatform/BP_DisappearPlatform.BP_DisappearPlatform_C"))
  (`|SpawnActorFromClass` (select `int` (`KismetMathLibrary.RandomIntegerInRange` 0 11) :`0` "/Game/Thomas/BPs/Bonus/BP_CarBoost.BP_CarBoost_C" :`1` "/Game/Thomas/BPs/Bonus/JumpBoost/BP_JumpBoost.BP_JumpBoost_C" :`2` "/Game/Thomas/BPs/Bonus/BP_StarBoost.BP_StarBoost_C" :`3` "/Game/Thomas/BPs/Bonus/IceBottle/BP_IceEffect.BP_IceEffect_C" :`4` "/Game/Thomas/BPs/Bonus/Ressort/BP_Resssort.BP_Resssort_C" :`5` "/Game/Thomas/BPs/Bonus/BP_Marteau.BP_Marteau_C" :`6` "/Game/Thomas/BPs/Bonus/BP_SpeedBoost.BP_SpeedBoost_C" :`7` "/Game/Thomas/BPs/Bonus/Ralentissement/BP_PotionRalentissement.BP_PotionRalentissement_C" :`8` "/Game/Thomas/BPs/Bonus/CameraReverse/BP_ReverseCamera.BP_ReverseCamera_C" :`9` "/Game/Thomas/BPs/Bonus/BP_CameraBlackAndWhite.BP_CameraBlackAndWhite_C" :`10` "/Game/Thomas/BPs/Bonus/Freddy/BP_Freddy.BP_Freddy_C" :`11` "/Game/Thomas/BPs/Bonus/BP_BigHammer.BP_BigHammer_C" :!type "Actor Class Reference") (`SceneComponent.K2_GetComponentToWorld` (`/Game/Thomas/BPs/DIsappearPlatform/BP_DisappearPlatform.DefaultSceneRoot` (`|GetArrayItem` _outactors (`KismetMathLibrary.RandomIntegerInRange` 0 120)))) "Undefined" "OverrideRootScale" null null))

(event `SpawnJACK`
  ;[0.376 0 0.03951] JACK EVENT
  (bind _outactors (`GameplayStatics.GetAllActorsOfClass` "/Game/Thomas/BPs/DIsappearPlatform/BP_DisappearPlatform.BP_DisappearPlatform_C"))
  (`|SpawnActorFromClass` "/Game/Thomas/BPs/Bonus/BP_JackInTheBox.BP_JackInTheBox_C" (`SceneComponent.K2_GetComponentToWorld` (`/Game/Thomas/BPs/DIsappearPlatform/BP_DisappearPlatform.DefaultSceneRoot` (`|GetArrayItem` _outactors (`KismetMathLibrary.RandomIntegerInRange` 0 120)))) "Undefined" "OverrideRootScale" null null))

(fn `FindPlayerStartByTag`
  (params (TagToFound :type Integer))
  (returns (PlayerStartFound :type "PlayerStart Object Reference"))
  (for _array_element (`self.PlayerStart`)
    (if (== (`PlayerStart.PlayerStartTag` _array_element) (`KismetStringLibrary.Conv_StringToName` (`KismetStringLibrary.Conv_IntToString` TagToFound)))
      (return _array_element)))
  (return null))

(fn `UserConstructionScript`)