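; BP_Platform is a platform actor that appears intended to vanish and return, but currently has no active effect.
; On BeginPlay it starts a looping timer whose event checks a Hit flag, with nothing wired to that branch.
; A disconnected chain of delays would hide the actor and disable its collision, then restore both, but it never runs.
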(event `self.ReceiveBeginPlay`
  (`KismetSystemLibrary.K2_SetTimerDelegate` (`|CreateDelegate` :!event `Timer`) 0.1 true))

(event `Timer`
  (if (`self.Hit?`)
    _))

(fn `UserConstructionScript`)