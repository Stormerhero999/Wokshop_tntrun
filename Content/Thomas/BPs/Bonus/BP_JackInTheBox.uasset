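; BP_JackInTheBox is a bonus trap actor that springs out and applies a malus to the first BP_Character overlapping its sphere.
; On BeginPlay it plays the spring-out animation while a timeline scales the trigger sphere and a ring mesh.
; On a hit it yaws toward the victim, calls JackMalus, plays its attack, then explodes and destroys itself.
; A delay started from the timeline update also destroys it after ten seconds.
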(event `self.ReceiveBeginPlay`
  (`SkeletalMeshComponent.PlayAnimation` (`self.Mesh`) "/Game/Anais/Animations/JackInTheBox_Springout_animation.JackInTheBox_Springout_animation" false)
  (bind (_direction _boxextend _ringextend) (`Timeline|Timeline_0` :!via `PlayFromStart`)
    (:`Update`
      (`SceneComponent.SetRelativeScale3D` (`self.Sphere`) (`KismetMathLibrary.Conv_DoubleToVector` _boxextend))
      (`SceneComponent.SetRelativeScale3D` (`self.StaticMesh`) (`KismetMathLibrary.MakeVector` _ringextend _ringextend 1.0))
      (`KismetSystemLibrary.Delay` 10.0)
      (`self.K2_DestroyActor`))))

(event `self.Sphere.OnComponentBeginOverlap`
  (params (OverlappedComponent :type "PrimitiveComponent Object Reference") (OtherActor :type "Actor Object Reference") (OtherComp :type "PrimitiveComponent Object Reference") (OtherBodyIndex :type Integer) (bFromSweep :type Boolean) (SweepResult :type "HitResult Structure (by ref)"))
  (bind _asbp_character (cast `/Game/Thomas/BPs/BP_Character` OtherActor))
  (`/Engine/EditorBlueprintResources/StandardMacros.DoOnce` false
    (:`Completed`
      (`self.K2_SetActorRotation` (`KismetMathLibrary.MakeRotator` 0.0 0.0 (.yaw (`KismetMathLibrary.FindLookAtRotation` (`self.K2_GetActorLocation`) (`self.K2_GetActorLocation` _asbp_character)))))
      (`/Game/Thomas/BPs/BP_Character.JackMalus` _asbp_character)
      (`SkeletalMeshComponent.PlayAnimation` (`self.Mesh`) "/Game/Anais/Animations/JackInTheBox_Attack_animation.JackInTheBox_Attack_animation" false)
      (`KismetSystemLibrary.Delay` 1.0)
      (`ActorComponent.Activate` (`self.Explode`) false)
      (`KismetSystemLibrary.Delay` 0.3)
      (`self.K2_DestroyActor`))))

(fn `UserConstructionScript`)