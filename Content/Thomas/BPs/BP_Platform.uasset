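; BP_Platform is a disappearing platform that hides and drops its collision two seconds after its Hit flag is set.
; Looping timers appear to drive a fast poll of Hit, which is set outside this graph, and Chrono, which sets DelayFinished after DelayPerPlatform.
; Before that deadline, a hit platform reappears five seconds after vanishing and re-arms its DoOnce.
; Afterwards, it stays gone.
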(event `Chrono`
  (set `self.Delay Finished?` true)
  (`KismetSystemLibrary.PrintString` "fini"))

(event `self.ReceiveBeginPlay`
  (`|ExecutionSequence`
    (:`then_0`
      (`KismetSystemLibrary.K2_SetTimerDelegate` (`|CreateDelegate` :!event `Chrono`) (`self.DelayPerPlatform`) true))
    (:`then_1`
      (`KismetSystemLibrary.K2_SetTimerDelegate` (`|CreateDelegate` :!event `Timer`) 0.1 true))))

(event `Timer`
  (if (`self.Hit?`)
    (`/Engine/EditorBlueprintResources/StandardMacros.DoOnce` false :!label _label
      (:`Completed`
        (if (`self.Delay Finished?`)
          (`KismetSystemLibrary.PrintString` "finish")
          (`KismetSystemLibrary.Delay` 2.0)
          (`self.SetActorHiddenInGame` true)
          (`self.SetActorEnableCollision` false)
          (set `self.Hit?` false)
          (else
            (`KismetSystemLibrary.Delay` 2.0)
            (`self.SetActorHiddenInGame` true)
            (`self.SetActorEnableCollision` false)
            (`KismetSystemLibrary.Delay` 5.0)
            (`self.SetActorHiddenInGame` false)
            (`self.SetActorEnableCollision` true)
            (set `self.Hit?` false)
            (goto _label :!via `Reset`)))))))

(fn `UserConstructionScript`)