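; BP_DisappearPlatform is a platform that repeatedly vanishes and reappears on a timed loop.
; After StartDelay on BeginPlay, it endlessly toggles the Cube's collision and hidden-in-game state, holding each state for FlickerTime.
; The construction script creates a dynamic material instance on the Cube and applies the Colour parameter, giving each placed instance its own tint.
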(event `self.ReceiveBeginPlay`
  (bind _cube (`self.Cube`))
  (bind _cube_2 (`self.Cube`))
  ;[1 1 1] Disappears and reappears all the time
  (`KismetSystemLibrary.Delay` (`self.StartDelay`))
  (`PrimitiveComponent.SetCollisionEnabled` _cube "NoCollision" :!label _label)
  (`SceneComponent.SetHiddenInGame` _cube true false)
  (`KismetSystemLibrary.Delay` (`self.FlickerTime`))
  (`PrimitiveComponent.SetCollisionEnabled` _cube_2 "QueryAndPhysics")
  (`SceneComponent.SetHiddenInGame` _cube_2 false false)
  (`KismetSystemLibrary.Delay` (`self.FlickerTime`))
  (goto _label))

(fn `UserConstructionScript`
  (bind _cube (`self.Cube`))
  ;[1 1 1] Change Color
  (bind _returnvalue (`PrimitiveComponent.CreateDynamicMaterialInstance` _cube 0 (`self.Source Material`) "None"))
  (`MaterialInstanceDynamic.SetVectorParameterValue` _returnvalue "Colour" (`self.Colour`))
  (`PrimitiveComponent.SetMaterial` _cube 0 _returnvalue))