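; BP_Canon is a cannon actor that periodically fires at a random player character.
; A looping timer started on BeginPlay calls ShootPlayer, which picks among BP_Character actors using a hard-coded four-entry index range.
; It re-rolls while the pick is dead, with no exit if all are dead.
; For a living target, it snaps to face it and spawns a BP_Bullet at its Arrow component's transform.
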(event `self.ReceiveBeginPlay`
  (`KismetSystemLibrary.K2_SetTimerDelegate` (delegate `ShootPlayer`) 5.0 true))

(event `ShootPlayer`
  (bind _outactors (`GameplayStatics.GetAllActorsOfClass` "/Game/Thomas/BPs/BP_Character.BP_Character_C" :!label _label))
  (bind _output_get (set `self.Player` (`|GetArrayItem` _outactors (`KismetMathLibrary.RandomIntegerInRange` 0 3))))
  (if (not (`/Game/Thomas/BPs/BP_Character.PlayerDead` _output_get))
    (`self.K2_SetActorRotation` (`KismetMathLibrary.FindLookAtRotation` (`self.K2_GetActorLocation`) (`self.K2_GetActorLocation` (`self.Player`))))
    (`|SpawnActorFromClass` "/Game/Thomas/BPs/Canon/BP_Bullet.BP_Bullet_C" (`SceneComponent.K2_GetComponentToWorld` (`self.Arrow`)) "Undefined" "OverrideRootScale" null null)
    (else
      (goto _label))))

(fn `UserConstructionScript`)