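; Game mode that spawns and possesses a character for each local player when play begins, up to a configured player count.
; BeginPlay spawns BP_Character for player 0, then creates any missing local controllers and spawns and possesses a pawn for each.
; Spawn points are PlayerStarts whose tag matches the player index.
; Player 0's view target is then set to the level's BP_Cam, giving a shared camera.
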(event `self.ReceiveBeginPlay`
  (bind _outactors (`GameplayStatics.GetAllActorsOfClass` "/Script/Engine.PlayerStart"))
  (set `self.PlayerStart` _outactors)
  (bind _returnvalue (`|SpawnActorFromClass` "/Game/Thomas/BPs/BP_Character.BP_Character_C" (`self.GetTransform` (`self.FindPlayerStartByTag` 0)) "Undefined" "OverrideRootScale" null null))
  (`Controller.Possess` (`GameplayStatics.GetPlayerController` 0) _returnvalue)
  (for _index (range 1 (`self.NbPlayerToSpawn`))
    (bind _returnvalue_2 (`GameplayStatics.GetPlayerControllerFromID` _index))
    (`/Engine/EditorBlueprintResources/StandardMacros.IsValid` _returnvalue_2
      (:`Is Valid`
        _)
      (:`Is Not Valid`
        (`GameplayStatics.CreatePlayer` _index)))
    (bind _returnvalue_3 (`|SpawnActorFromClass` "/Game/Thomas/BPs/BP_Character.BP_Character_C" (`self.GetTransform` (`self.FindPlayerStartByTag` _index)) "Undefined" "OverrideRootScale" null null))
    (`Controller.Possess` _returnvalue_2 _returnvalue_3))
  (bind _returnvalue_4 (`GameplayStatics.GetActorOfClass` "/Game/Thomas/BPs/BP_Cam.BP_Cam_C"))
  (`PlayerController.SetViewTargetWithBlend` (`GameplayStatics.GetPlayerController` 0) _returnvalue_4 0.0 "VTBlend_Linear" 0.0 false))

(fn `FindPlayerStartByTag`
  (params (TagToFound :type Integer))
  (returns (PlayerStartFound :type "PlayerStart Object Reference"))
  (for _array_element (`self.PlayerStart`)
    (if (== (`PlayerStart.PlayerStartTag` _array_element) (`KismetStringLibrary.Conv_StringToName` (`KismetStringLibrary.Conv_IntToString` TagToFound)))
      (return _array_element)))
  (return null))

(fn `UserConstructionScript`)