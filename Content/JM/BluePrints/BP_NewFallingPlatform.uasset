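; Falling platform actor that, despite the name, vanishes in place by hiding its cube mesh and disabling collision, then returns on rebirth.
; Custom events forward to functions that chain one-shot timers for countdown, near-death, death and respawn, though timer bindings are not shown.
; Material setters provide color warning stages.
; Three near-duplicate timer sets have separate delay and respawn variables, with debug prints on death and rebirth.
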(event `SetMaterAlive`
  (`PrimitiveComponent.SetMaterial` (`self.CubePlatform`) 0 (`self.MaterialAlive`)))

(event `SetMaterYell`
  (`PrimitiveComponent.SetMaterial` (`self.CubePlatform`) 0 (`self.MaterialYellow`)))

(event `SetMaterNear`
  (`PrimitiveComponent.SetMaterial` (`self.CubePlatform`) 0 (`self.MaterialNear`))
  (`KismetMaterialLibrary.SetVectorParameterValue` null "None" (`self.Parameter Value`)))

(event `Set0ce`
  (`KismetSystemLibrary.K2_SetTimerDelegate` (`|CreateDelegate` :!event `Neardeath`) (- (`self.Time`) 9.9)))

(event `SetMaterDaOr`
  (`PrimitiveComponent.SetMaterial` (`self.CubePlatform`) 0 (`self.MaterialDarkOrange`)))

(event `Set1ce`
  (`KismetSystemLibrary.K2_SetTimerDelegate` (`|CreateDelegate` :!event `NearDeath1`) (- (`self.Time1`) 9.9)))

(event `SetMaterDeath`
  (`PrimitiveComponent.SetMaterial` (`self.CubePlatform`) 0 (`self.MaterialDeath`)))

(event `Set2ce`
  (`KismetSystemLibrary.K2_SetTimerDelegate` (`|CreateDelegate` :!event `NearDeath2`) (- (`self.Time2`) 9.9)))

(event `PlateformDeath`
  (`KismetSystemLibrary.PrintString` "Ded")
  (`SceneComponent.SetHiddenInGame` (`self.CubePlatform`) true false)
  (`PrimitiveComponent.SetCollisionEnabled` (`self.CubePlatform`) "NoCollision")
  (`KismetSystemLibrary.K2_SetTimerDelegate` (`|CreateDelegate` :!event `PlatformRebirth`) (`self.RespawnT`)))

(event `Neardeath`
  (`KismetSystemLibrary.K2_SetTimerDelegate` (`|CreateDelegate` :!event `SetMaterAlive`) 0.9)
  (`KismetSystemLibrary.K2_SetTimerDelegate` (`|CreateDelegate` :!event `SetMaterYell`) 3.0)
  (`KismetSystemLibrary.K2_SetTimerDelegate` (`|CreateDelegate` :!event `SetMaterNear`) 5.0)
  (`KismetSystemLibrary.K2_SetTimerDelegate` (`|CreateDelegate` :!event `SetMaterDaOr`) 7.0)
  (`KismetSystemLibrary.K2_SetTimerDelegate` (`|CreateDelegate` :!event `SetMaterDeath`) 9.0)
  (`KismetSystemLibrary.K2_SetTimerDelegate` (`|CreateDelegate` :!event `PlateformDeath`) 10.0))

(event `PlateformDeath1`
  (`KismetSystemLibrary.PrintString` "Ded")
  (`SceneComponent.SetHiddenInGame` (`self.CubePlatform`) true false)
  (`PrimitiveComponent.SetCollisionEnabled` (`self.CubePlatform`) "NoCollision")
  (`KismetSystemLibrary.K2_SetTimerDelegate` (`|CreateDelegate` :!event `PlatformRebirth`) (`self.RespawnT1`)))

(event `NearDeath1`
  (`KismetSystemLibrary.K2_SetTimerDelegate` (`|CreateDelegate` :!event `SetMaterAlive`) 0.9)
  (`KismetSystemLibrary.K2_SetTimerDelegate` (`|CreateDelegate` :!event `SetMaterYell`) 3.0)
  (`KismetSystemLibrary.K2_SetTimerDelegate` (`|CreateDelegate` :!event `SetMaterNear`) 5.0)
  (`KismetSystemLibrary.K2_SetTimerDelegate` (`|CreateDelegate` :!event `SetMaterDaOr`) 7.0)
  (`KismetSystemLibrary.K2_SetTimerDelegate` (`|CreateDelegate` :!event `SetMaterDeath`) 9.0)
  (`KismetSystemLibrary.K2_SetTimerDelegate` (`|CreateDelegate` :!event `PlateformDeath1`) 2.0))

(event `NearDeath2`
  (`KismetSystemLibrary.K2_SetTimerDelegate` (`|CreateDelegate` :!event `SetMaterAlive`) 0.9)
  (`KismetSystemLibrary.K2_SetTimerDelegate` (`|CreateDelegate` :!event `SetMaterYell`) 3.0)
  (`KismetSystemLibrary.K2_SetTimerDelegate` (`|CreateDelegate` :!event `SetMaterNear`) 5.0)
  (`KismetSystemLibrary.K2_SetTimerDelegate` (`|CreateDelegate` :!event `SetMaterDaOr`) 7.0)
  (`KismetSystemLibrary.K2_SetTimerDelegate` (`|CreateDelegate` :!event `SetMaterDeath`) 9.0)
  (`KismetSystemLibrary.K2_SetTimerDelegate` (`|CreateDelegate` :!event `PlateformDeath2`) 2.0))

(event `PlateformDeath2`
  (`KismetSystemLibrary.PrintString` "Ded")
  (`SceneComponent.SetHiddenInGame` (`self.CubePlatform`) true false)
  (`PrimitiveComponent.SetCollisionEnabled` (`self.CubePlatform`) "NoCollision")
  (`KismetSystemLibrary.K2_SetTimerDelegate` (`|CreateDelegate` :!event `PlatformRebirth`) (`self.RespawnT2`)))

(event `PlatformRebirth`
  (`KismetSystemLibrary.PrintString` "Alive")
  (`PrimitiveComponent.SetMaterial` (`self.CubePlatform`) 0 (`self.MaterialLive`))
  (`SceneComponent.SetHiddenInGame` (`self.CubePlatform`) false false)
  (`PrimitiveComponent.SetCollisionEnabled` (`self.CubePlatform`) "QueryAndPhysics"))

(fn `UserConstructionScript`)