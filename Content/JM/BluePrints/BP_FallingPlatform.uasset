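; BP_FallingPlatform is a platform that drops away after the player character steps on it, then returns.
; An overlap on Bhru runs a DoOnce-gated delay chain: dip slightly, change material as warning, hide and disable collision, then restore and reset.
; BeginPlay starts a one-shot timer.
; A separate PlateformDeath event sets StopSpawn, which feeds the DoOnce, and destroys the actor.
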(event `self.ReceiveBeginPlay`
  (bind _returnvalue (`KismetSystemLibrary.K2_SetTimerDelegate` (`|CreateDelegate` :!event `PlateformDeath`) (`self.Time`)))
  (set `self.TimerHandle` _returnvalue))

(event `self.Bhru.OnComponentBeginOverlap`
  (params (OverlappedComponent :type "PrimitiveComponent Object Reference") (OtherActor :type "Actor Object Reference") (OtherComp :type "PrimitiveComponent Object Reference") (OtherBodyIndex :type Integer) (bFromSweep :type Boolean) (SweepResult :type "HitResult Structure (by ref)"))
  (cast `/Game/Thomas/BPs/BP_Character` OtherActor)
  (`KismetSystemLibrary.PrintString` "Act")
  (`/Engine/EditorBlueprintResources/StandardMacros.DoOnce` (stale `PlateformDeath` _output_get) :!label _label
    (:`Completed`
      (`self.K2_AddActorLocalOffset` (0.0 0.0 -3.0) true)
      (`KismetSystemLibrary.Delay` 0.2)
      (`PrimitiveComponent.SetMaterial` (`self.CubePlatform`) 0 "/Engine/EngineDebugMaterials/VertexColorViewMode_GreenOnly.VertexColorViewMode_GreenOnly")
      (`KismetSystemLibrary.Delay` 1.5)
      (`PrimitiveComponent.SetMaterial` (`self.CubePlatform`) 0 "/Engine/EngineDebugMaterials/VertexColorViewMode_RedOnly.VertexColorViewMode_RedOnly")
      (`KismetSystemLibrary.Delay` 0.5)
      (`PrimitiveComponent.SetCollisionEnabled` (`self.CubePlatform`) "NoCollision")
      (`self.SetActorHiddenInGame` true)
      (`KismetSystemLibrary.Delay` 3.0)
      (`PrimitiveComponent.SetCollisionEnabled` (`self.CubePlatform`) "QueryAndPhysics")
      (`self.SetActorHiddenInGame` false)
      (`PrimitiveComponent.SetMaterial` (`self.CubePlatform`) 0 "/Game/JM/StaticMesh_Materials/lambert1.lambert1")
      (`self.K2_AddActorLocalOffset` (0.0 0.0 3.0))
      (goto _label :!via `Reset`))))

(event `PlateformDeath`
  (bind _output_get (set `self.StopSpawn` true))
  (if _output_get
    (`KismetSystemLibrary.PrintString` "Ded")
    (`self.K2_DestroyActor`)))

(fn `UserConstructionScript`)