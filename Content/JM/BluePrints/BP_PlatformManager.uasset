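; BP_PlatformManager periodically triggers one of three randomly chosen sets on the level's falling platforms.
; On BeginPlay it gathers all BP_NewFallingPlatform actors and starts a looping timer whose interval is the Loop variable.
; A random roll in launchRSet calls Set0ce, Set1ce or Set2ce on those platforms.
; A step that would shorten Loop is present but never runs.
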(event `self.ReceiveBeginPlay`
  (bind _outactors (`GameplayStatics.GetAllActorsOfClass` "/Game/JM/BluePrints/BP_NewFallingPlatform.BP_NewFallingPlatform_C"))
  (set `self.PlatformInst` _outactors)
  (`KismetSystemLibrary.K2_SetTimerDelegate` (`|CreateDelegate` :!event `launchRSet`) (`self.Loop`) true))

(event `launchRSet`
  (bind _platforminst (`self.PlatformInst`))
  (bind _output_get (set `self.Rset` (`KismetMathLibrary.RandomIntegerInRange` 0 2)))
  (switch `int` _output_get
    (:`0`
      (`/Game/JM/BluePrints/BP_NewFallingPlatform.Set0ce` _platforminst))
    (:`1`
      (`/Game/JM/BluePrints/BP_NewFallingPlatform.Set1ce` _platforminst))
    (:`2`
      (`/Game/JM/BluePrints/BP_NewFallingPlatform.Set2ce` _platforminst))))

(fn `UserConstructionScript`)